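; BP_Enemy is an enemy actor that flies in a straight line and kills the player on contact.
; On BeginPlay it randomly, weighted by TraceRate, either looks up BP_Player to set a one-time homing direction or uses its own forward vector.
; Tick moves it along that fixed direction at MoveSpeed without sweeping.
; Overlapping BP_Player destroys the player, spawns an explosion emitter and destroys the enemy.
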(event Collision|EventActorBeginOverlap
  (params (OtherActor :type Actor%20Object%20Reference))
  (bind _asbp_player (Utilities|Casting|CastToBP_Player OtherActor))
  (Actor|DestroyActor _asbp_player)
  (Effects|SpawnEmitteratLocation "/Game/StarterContent/Particles/P_Explosion.P_Explosion" (Transformation|GetActorLocation))
  (Actor|DestroyActor))

(event EventTick
  (params (DeltaSeconds :type Float%20%28single-precision%29))
  (Transformation|SetActorLocation (+ (Transformation|GetActorLocation) (* (* (Variables|Default|GetDirection) (Variables|Default|GetMoveSpeed)) DeltaSeconds)) false false))

(event EventBeginPlay
  ;[1 1 1] 적 생성시 캐릭터 위치 찾기
  (if (<= (Math|Random|RandomFloatinRange 0.0 1.0) (Variables|Default|GetTraceRate))
    (bind _returnvalue (Actor|GetActorOfClass "/Game/BluePrints/BP_Player.BP_Player_C"))
    (Utilities|IsValid _returnvalue
      (:Is%20Valid
        (Variables|Default|SetDirection (Math|Vector|Normalize (- (Transformation|GetActorLocation) (Transformation|GetActorLocation))))))
    (else
      (Variables|Default|SetDirection (Transformation|GetActorForwardVector)))))

(fn ConstructionScript)